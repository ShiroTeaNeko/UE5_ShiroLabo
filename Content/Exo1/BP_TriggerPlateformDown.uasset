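; Trigger box that sends a referenced elevator down one floor when the third-person character enters it.
; Overlap decrements the elevator's floor index within clamped bounds, then restarts a timeline.
; Each timeline update passes MoveToDirection a lerp from the cube's current world location toward that floor's transform location, re-reading the start point every tick.
; End overlap only casts, and an IsUp-based GoUp/GoDown branch is left unconnected.
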(event `self.Box.OnComponentBeginOverlap`
  (params (OverlappedComponent :type "PrimitiveComponent Object Reference") (OtherActor :type "Actor Object Reference") (OtherComp :type "PrimitiveComponent Object Reference") (OtherBodyIndex :type Integer) (bFromSweep :type Boolean) (SweepResult :type "HitResult Structure (by ref)"))
  (bind _elevator (`self.Elevator`))
  (bind _elevator_2 (`self.Elevator`))
  (cast `/Game/Exo1/BP_ThirdPersonCharacter` OtherActor)
  (bind _output_get (set `/Game/Exo1/platform.actualFloor` (`KismetMathLibrary.Clamp` (- (`/Game/Exo1/platform.actualFloor` _elevator_2) 1) 0 (`/Game/Exo1/platform.numberFloorMax` _elevator_2)) _elevator_2))
  (bind (_direction _alpha) (`Timeline|Timeline` :!via `PlayFromStart`)
    (:`Update`
      (`/Game/Exo1/platform.MoveToDirection` _elevator (`KismetMathLibrary.VLerp` (`SceneComponent.K2_GetComponentLocation` (`/Game/Exo1/platform.Cube` _elevator)) (`KismetMathLibrary.TransformLocation` (`|GetArrayItem` (`/Game/Exo1/platform.Floors` _elevator_2) _output_get)) _alpha)))))

(event `self.Box.OnComponentEndOverlap`
  (params (OverlappedComponent :type "PrimitiveComponent Object Reference") (OtherActor :type "Actor Object Reference") (OtherComp :type "PrimitiveComponent Object Reference") (OtherBodyIndex :type Integer))
  (cast `/Game/Exo1/BP_ThirdPersonCharacter` OtherActor))

(fn `UserConstructionScript`)