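; BP_Plane is a player-controlled, physics-driven plane that constantly flies forward.
; Each Tick blends the capsule's linear velocity toward its forward vector at a clamped, delta-time-scaled speed that normally stays at the minimum.
; Tick also damps spin by adding a fraction of the negated angular velocity.
; Roll, Turn and LookUp axes apply scaled acceleration torques around the forward, up and right vectors respectively.
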(event `self.ReceiveBeginPlay`)

(event `self.ReceiveTick`
  (params (DeltaSeconds :type "Float (single-precision)"))
  (bind _capsulecomponent (`self.CapsuleComponent`))
  (bind _capsulecomponent_2 (`self.CapsuleComponent`))
  (bind _returnvalue (`PrimitiveComponent.GetPhysicsLinearVelocity` _capsulecomponent "None"))
  (`PrimitiveComponent.SetPhysicsLinearVelocity` _capsulecomponent (`KismetMathLibrary.VLerp` _returnvalue (* (`KismetMathLibrary.FClamp` (* DeltaSeconds 3000.0) 3000.0 10000.0) (`self.GetActorForwardVector`)) 0.1) false "None")
  (`PrimitiveComponent.SetPhysicsAngularVelocityInDegrees` _capsulecomponent_2 (/ (`KismetMathLibrary.NegateVector` (`PrimitiveComponent.GetPhysicsAngularVelocityInDegrees` _capsulecomponent_2 "None")) (20.0 20.0 20.0)) true "None"))

(event `InputAxis|Roll`
  (params (AxisValue :type "Float (single-precision)"))
  (`PrimitiveComponent.AddTorqueInDegrees` (`self.CapsuleComponent`) (`KismetMathLibrary.VLerp` (0.0 0.0 0.0) (* (* AxisValue 4000.0) (`self.GetActorForwardVector`)) 0.1) "None" true))

(event `InputAxis|Turn`
  (params (AxisValue :type "Float (single-precision)"))
  (`PrimitiveComponent.AddTorqueInDegrees` (`self.CapsuleComponent`) (`KismetMathLibrary.VLerp` (0.0 0.0 0.0) (* (* AxisValue 1500.0) (`self.GetActorUpVector`)) 0.1) "None" true))

(event `InputAxis|LookUp`
  (params (AxisValue :type "Float (single-precision)"))
  (`PrimitiveComponent.AddTorqueInDegrees` (`self.CapsuleComponent`) (`KismetMathLibrary.VLerp` (0.0 0.0 0.0) (* (* AxisValue 3000.0) (`self.GetActorRightVector`)) 0.1) "None" true))

(fn `UserConstructionScript`)